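; BP_NetStat is a functional test that toggles the network stats display for a timed window.
; On test start it runs the "stat net" console command, waits, then runs it again to toggle the stats back.
; After a short further delay it always finishes as Succeeded with a profile-save message, without checking or saving any values itself.
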(event `self.ReceiveStartTest`
  (`parent.ReceiveStartTest`)
  (`KismetSystemLibrary.ExecuteConsoleCommand` "stat net" null)
  (`KismetSystemLibrary.Delay` 15.0)
  (`KismetSystemLibrary.ExecuteConsoleCommand` "stat net" null)
  (`KismetSystemLibrary.Delay` 1.0)
  (`self.FinishTest` "Succeeded" "NetProfale Save"))

(fn `UserConstructionScript`
  (`parent.UserConstructionScript`))