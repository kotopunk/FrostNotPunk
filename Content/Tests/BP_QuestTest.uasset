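; BP_QuestTest is a functional test that records an Unreal trace over a fixed time window.
; On test start it runs the Trace.Start console command, waits on a delay, then runs Trace.Stop and finishes as Succeeded.
; It makes no assertions, so it serves as a timed capture rather than a pass/fail check.
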(event `self.ReceiveStartTest`
  (`parent.ReceiveStartTest`)
  (`KismetSystemLibrary.ExecuteConsoleCommand` "Trace.Start" null)
  (`KismetSystemLibrary.Delay` 15.0)
  (`KismetSystemLibrary.ExecuteConsoleCommand` "Trace.Stop" null)
  (`self.FinishTest` "Succeeded"))

(event `self.ReceiveTick`
  (params (DeltaSeconds :type "Float (single-precision)"))
  (`parent.ReceiveTick` DeltaSeconds))

(fn `UserConstructionScript`
  (`parent.UserConstructionScript`))