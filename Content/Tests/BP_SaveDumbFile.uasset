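; Functional test Blueprint that attempts to record a stats capture file while MainMap loads and runs.
; StartTest issues "stat startfile", opens MainMap, waits on a fixed delay, then issues a stop command and always finishes as Succeeded with no checks.
; The stop command is spelled "stat stoptfile" rather than "stat stopfile", and the delay and finish are sequenced after the level change in the same actor.
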(event `self.ReceiveStartTest`
  (`parent.ReceiveStartTest`)
  (`KismetSystemLibrary.ExecuteConsoleCommand` "stat startfile" null)
  (`GameplayStatics.OpenLevel` "MainMap")
  (`KismetSystemLibrary.Delay` 20.0)
  (`KismetSystemLibrary.ExecuteConsoleCommand` "stat stoptfile" null)
  (`self.FinishTest` "Succeeded"))

(fn `UserConstructionScript`
  (`parent.UserConstructionScript`))