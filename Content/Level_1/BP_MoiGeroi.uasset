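; Player character for what appears to be an endless game, with left/right axis movement and a Quinn/Manny skin applied on BeginPlay and OnRep_Skin.
; DeadFunction stops movement, pauses, saves through BP_EndlesSaveGame and shows WB_DeadScreen.
; It adds GameModeTest's CurrentPoint to saved coins and updates the high score when beaten, but a newly created save records only the high score.
; The pause-menu logic is disconnected.
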(event `self.ReceiveBeginPlay`
  ;[1 1 1] Chenge player skin
  (`self.UpdateMesh`))

(event `InputAxis|MoveRightLeft`
  (params (AxisValue :type "Float (single-precision)"))
  (`self.AddMovementInput` (0.0 1.0 0.0) AxisValue))

(fn `DeadFunction`
  (bind _returnvalue (`GameplayStatics.GetPlayerController` 0))
  (bind _saveslot (`self.SaveSlot`))
  (bind _saveslot_2 (`self.SaveSlot`))
  (bind _savever (`self.SaveVer`))
  (`PrimitiveComponent.SetSimulatePhysics` (`self.Mesh`) false)
  (`CharacterMovementComponent.DisableMovement` (`self.CharacterMovement`))
  (`GameplayStatics.SetGamePaused` true)
  (bind _asgame_mode_test (cast `/Game/Level_1/GameModeTest` (`GameplayStatics.GetGameMode`)))
  (bind _returnvalue_2 (`GameplayStatics.DoesSaveGameExist` _saveslot))
  (if _returnvalue_2
    (bind _returnvalue_3 (`GameplayStatics.LoadGameFromSlot` _saveslot))
    (bind _output_get (set `self.SaveVer` _returnvalue_3))
    (bind _asbp_endles_save_game (cast `/Game/Widgets/BP_EndlesSaveGame` _output_get))
    (bind _currentpoint (`/Game/Level_1/GameModeTest.CurrentPoint` _asgame_mode_test))
    (if (> _currentpoint (`/Game/Widgets/BP_EndlesSaveGame.HighsCoreValue` _asbp_endles_save_game))
      (set `/Game/Widgets/BP_EndlesSaveGame.CurrentCoins` (+ (`/Game/Widgets/BP_EndlesSaveGame.CurrentCoins` _asbp_endles_save_game) _currentpoint) _asbp_endles_save_game)
      (set `/Game/Widgets/BP_EndlesSaveGame.HighsCoreValue` _currentpoint _asbp_endles_save_game)
      (`GameplayStatics.SaveGameToSlot` _savever _saveslot_2)
      (else
        (set `/Game/Widgets/BP_EndlesSaveGame.CurrentCoins` (+ (`/Game/Widgets/BP_EndlesSaveGame.CurrentCoins` _asbp_endles_save_game) _currentpoint) _asbp_endles_save_game)
        (`GameplayStatics.SaveGameToSlot` _savever _saveslot_2)))
    (else
      (bind _returnvalue_4 (`GameplayStatics.CreateSaveGameObject` "/Game/Widgets/BP_EndlesSaveGame.BP_EndlesSaveGame_C"))
      (bind _output_get_2 (set `self.SaveVer` _returnvalue_4))
      (bind _asbp_endles_save_game_2 (cast `/Game/Widgets/BP_EndlesSaveGame` _output_get_2))
      (set `/Game/Widgets/BP_EndlesSaveGame.HighsCoreValue` _currentpoint _asbp_endles_save_game_2)
      (`GameplayStatics.SaveGameToSlot` _savever _saveslot_2)))
  (set `PlayerController.bShowMouseCursor` true _returnvalue)
  (bind _returnvalue_5 (`|CreateWidget` "/Game/Widgets/WidgetBluePrints/WB_DeadScreen.WB_DeadScreen_C" _returnvalue))
  (bind _output_get_3 (set `self.DeadScreenRef` _returnvalue_5))
  (`UserWidget.AddToViewport` _output_get_3 0))

(fn `OnRep_Skin`
  (`self.UpdateMesh`))

(fn `sss`
  (returns (NewParam :type "SkeletalMesh Object Reference"))
  (return null))

(fn `UpdateMesh`
  (`SkeletalMeshComponent.SetSkeletalMeshAsset` (`self.Mesh`) (select `int` (`self.Skin`) :`0` "/Game/Level_1/Mannequins/Meshes/SKM_Quinn.SKM_Quinn" :`1` "/Game/Level_1/Mannequins/Meshes/SKM_Manny.SKM_Manny" :!type "SkeletalMesh Object Reference")))

(fn `UserConstructionScript`)