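; BP_Dogonyator is a Level 1 actor, apparently a boss, whose health runs down on a timer until it is destroyed.
; BeginPlay adds a WB_BossHP widget to the viewport.
; Tick uses a one-second Delay to decrement MaxHP itself, copy it into CurrentHP and print the value.
; When CurrentHP equals exactly zero, it destroys the actor and removes the widget.
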(event `self.ReceiveBeginPlay`
  (bind _returnvalue (`|CreateWidget` "/Game/Widgets/WidgetBluePrints/WB_BossHP.WB_BossHP_C"))
  (`UserWidget.AddToViewport` _returnvalue 0))

(event `self.ReceiveTick`
  (params (DeltaSeconds :type "Float (single-precision)"))
  (`KismetSystemLibrary.Delay` 1.0)
  (bind _result (`/Engine/EditorBlueprintResources/StandardMacros.DecrementFloat` (`self.MaxHP`))
    (:`  `
      (bind _output_get (set `self.Current HP` _result))
      (`KismetSystemLibrary.PrintString` (`KismetStringLibrary.Conv_DoubleToString` _output_get))
      (if (== (`self.Current HP`) 0.0)
        (`self.K2_DestroyActor`)
        (`Widget.RemoveFromParent` (stale `self.ReceiveBeginPlay` _returnvalue))))))

(fn `UserConstructionScript`)