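; BP_EndGame2 is the countdown timer for the Game2 mode, ending the run when minutes and seconds reach zero.
; Tick uses a one-second Delay as a gate to decrement the timer.
; TimeIsOver pauses, updates CurrentCoins in the endless save by adding Coins, and shows the dead screen with best/current rows hidden.
; Getters expose minutes and seconds, while duration, speed and Gans getters return zero.
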(event `self.ReceiveBeginPlay`)

(event `self.ReceiveTick`
  (params (DeltaSeconds :type "Float (single-precision)"))
  (`KismetSystemLibrary.Delay` 1.0)
  (if (== (`self.Seconds`) 0)
    (if (== (`self.Minutes`) 0)
      (`self.TimeIsOver`)
      (else
        (set `self.Seconds` 59)
        (set `self.Minutes` (- (`self.Minutes`) 1))))
    (else
      (set `self.Seconds` (- (`self.Seconds`) 1)))))

(fn `GetDuration`
  (returns (Duration :type "Float (double-precision)"))
  (return 0.0))

(fn `GetGans`
  (returns (Gans :type "Float (double-precision)"))
  (return 0.0))

(fn `GetMinutes`
  (returns (Minut :type Integer))
  (return (`self.Minutes`)))

(fn `GetSeconds`
  (returns (Sec :type Integer))
  (return (`self.Seconds`)))

(fn `GetSpeed`
  (returns (Speed :type "Float (double-precision)"))
  (return 0.0))

(fn `TimeIsOver`
  (bind _returnvalue (`GameplayStatics.GetPlayerController` 0))
  (`GameplayStatics.SetGamePaused` true)
  (bind _returnvalue_2 (`GameplayStatics.LoadGameFromSlot` (`self.SaveSlot`)))
  (bind _output_get (set `self.SaveRef` _returnvalue_2))
  (bind _asbp_endles_save_game (cast `/Game/Widgets/BP_EndlesSaveGame` _output_get))
  (set `/Game/Widgets/BP_EndlesSaveGame.CurrentCoins` (+ (`/Game/Widgets/BP_EndlesSaveGame.Coins` _asbp_endles_save_game) (`/Game/Widgets/BP_EndlesSaveGame.CurrentCoins` _asbp_endles_save_game)) _asbp_endles_save_game)
  (`GameplayStatics.SaveGameToSlot` (`self.SaveRef`) (`self.SaveSlot`))
  (set `PlayerController.bShowMouseCursor` true _returnvalue)
  (bind _returnvalue_3 (`|CreateWidget` "/Game/Widgets/WidgetBluePrints/WB_DeadScreen.WB_DeadScreen_C" _returnvalue))
  (`UserWidget.AddToViewport` _returnvalue_3 0)
  (`Widget.SetVisibility` (`/Game/Widgets/WidgetBluePrints/WB_DeadScreen.HorizontalBox_Best` _returnvalue_3) "Hidden")
  (`Widget.SetVisibility` (`/Game/Widgets/WidgetBluePrints/WB_DeadScreen.HorizontalBox_Current` _returnvalue_3) "Hidden")
  (`WidgetBlueprintLibrary.SetInputMode_UIOnlyEx` (`GameplayStatics.GetPlayerController` 0) _returnvalue_3))

(fn `UserConstructionScript`)