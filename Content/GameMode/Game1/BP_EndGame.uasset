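; BP_EndGame handles game over for the endless mode, calling EndGame from Tick three seconds after IsDead is set by NewBoll.
; EndGame pauses the game, banks coins and any new high score into the endless save, then shows the dead-screen widget.
; It also rebuilds the saved leaderboard, inserting the current score once via DoOnce before the first lower-or-equal entry and dropping existing ties.
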(event `self.ReceiveBeginPlay`)

(event `self.ReceiveTick`
  (params (DeltaSeconds :type "Float (single-precision)"))
  (if (`self.is dead`)
    (`KismetSystemLibrary.Delay` 3.0)
    (`self.EndGame`)))

(fn `EndGame`
  (bind _returnvalue (`GameplayStatics.GetPlayerController` 0))
  (bind _saveslot (`self.SaveSlot`))
  (bind _saveref (`self.SaveRef`))
  (`|ExecutionSequence`
    (:`then_0`
      (`GameplayStatics.SetGamePaused` true)
      (bind _asgame_mode_test (cast `/Game/GameMode/Game1/GameModeTest` (`GameplayStatics.GetGameMode`)))
      (bind _returnvalue_2 (`GameplayStatics.LoadGameFromSlot` (`self.SaveSlot`)))
      (bind _output_get (set `self.SaveRef` _returnvalue_2))
      (bind _asbp_endles_save_game (cast `/Game/Widgets/BP_EndlesSaveGame` _output_get))
      (bind _currentpoint (`/Game/GameMode/Game1/GameModeTest.CurrentPoint` _asgame_mode_test))
      (if (> _currentpoint (`/Game/Widgets/BP_EndlesSaveGame.HighsCoreValue` _asbp_endles_save_game))
        (bind _coins (`/Game/Widgets/BP_EndlesSaveGame.Coins` _asbp_endles_save_game))
        (set `/Game/Widgets/BP_EndlesSaveGame.CurrentCoins` (+ _coins (`/Game/Widgets/BP_EndlesSaveGame.CurrentCoins` _asbp_endles_save_game)) _asbp_endles_save_game)
        (set `/Game/Widgets/BP_EndlesSaveGame.HighsCoreValue` _currentpoint _asbp_endles_save_game)
        (`GameplayStatics.SaveGameToSlot` _saveref _saveslot)
        (else
          (set `/Game/Widgets/BP_EndlesSaveGame.CurrentCoins` (+ (`/Game/Widgets/BP_EndlesSaveGame.CurrentCoins` _asbp_endles_save_game) _coins) _asbp_endles_save_game)
          (`GameplayStatics.SaveGameToSlot` _saveref _saveslot)))
      (set `PlayerController.bShowMouseCursor` true _returnvalue)
      (bind _returnvalue_3 (`|CreateWidget` "/Game/Widgets/WidgetBluePrints/WB_DeadScreen.WB_DeadScreen_C" _returnvalue))
      (`UserWidget.AddToViewport` _returnvalue_3 0)
      (`WidgetBlueprintLibrary.SetInputMode_UIOnlyEx` (`GameplayStatics.GetPlayerController` 0) _returnvalue_3))
    (:`then_1`
      (bind _returnvalue_4 (`GameplayStatics.LoadGameFromSlot` (`self.Slot Name`)))
      (bind _asscore_save (cast `/Game/Level_1/ScoreSave` _returnvalue_4)
        (:`then`
          (for _array_element (`/Game/Level_1/ScoreSave.PlayerScores` _asscore_save)
            (`|ExecutionSequence`
              (:`then_0`
                (bind (_name _score) (break `/Game/Level_1/PlayerScore` _array_element))
                (if (<= _score _currentpoint)
                  (`/Engine/EditorBlueprintResources/StandardMacros.DoOnce` false :!label _label
                    (:`Completed`
                      (`KismetArrayLibrary.Array_Add` (`self.Temp`) (make `/Game/Level_1/PlayerScore` (`/Game/Widgets/BP_EndlesSaveGame.PlayerName` _asbp_endles_save_game) _currentpoint))))))
              (:`then_1`
                (if (not (== _score _currentpoint))
                  (`KismetArrayLibrary.Array_Add` (`self.Temp`) _array_element)))))
          (`|ExecutionSequence`
            (:`then_0`
              (goto _label))
            (:`then_1`
              (bind _returnvalue_5 (`GameplayStatics.CreateSaveGameObject` "/Game/Level_1/ScoreSave.ScoreSave_C" :!label _label_2))
              (bind _asscore_save_2 (cast `/Game/Level_1/ScoreSave` _returnvalue_5))
              (set `/Game/Level_1/ScoreSave.PlayerScores` (`self.Temp`) _asscore_save_2)
              (`GameplayStatics.SaveGameToSlot` _returnvalue_5 (`self.Slot Name`)))))
        (:`CastFailed`
          (`|ExecutionSequence`
            (:`then_0`
              (goto _label))
            (:`then_1`
              (goto _label_2))))))))

(fn `IsDead`
  (returns (NewParam :type Boolean))
  (return false))

(fn `NewBoll`
  (returns (NewParam :type Boolean))
  (set `self.is dead` true)
  (return false))

(fn `UserConstructionScript`)