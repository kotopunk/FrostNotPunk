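; BP_SpawnMars is an enemy spawner that repeatedly spawns BP_Mars at its own location at a shrinking interval.
; BeginPlay waits briefly, then spawns and loops back after a RespawnTime delay, wired through a single-iteration for loop.
; In parallel, Tick uses a similar delayed loop to periodically decrement RespawnTime until it reaches a lower limit, so spawns become more frequent.
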(event `self.ReceiveBeginPlay`
  (`KismetSystemLibrary.Delay` 3.0)
  (`|SpawnActorFromClass` "/Game/Assets/Enemies/PlanetsEnemies/BP_Mars.BP_Mars_C" (`KismetMathLibrary.MakeTransform` (`self.K2_GetActorLocation`)) "Undefined" "OverrideRootScale" null null :!label _label)
  (`KismetSystemLibrary.Delay` (`self.RespawnTime`))
  (for _ (range 1)
    (goto _label)))

(event `self.ReceiveTick`
  (params (DeltaSeconds :type "Float (single-precision)"))
  (if (> (`self.RespawnTime`) 5.0) :!label _label_2
    (`KismetSystemLibrary.Delay` 10.0)
    (set `self.RespawnTime` (- (`self.RespawnTime`) 1.0))
    (for _ (range 1)
      (goto _label_2))))

(fn `UserConstructionScript`)