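; BP_PyrEnemy is a flying enemy that runs the FlyingAIBT behavior tree and spins its mesh on Tick.
; Each hit lowers MaxHP by one regardless of damage amount and copies it to CurrentHP.
; At zero it adds PointSelf to the saved Coins, then explodes with a random emitter.
; Overlapping a BP_Shield or SpaceStation deals damage to it and destroys the enemy without awarding coins.
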(event `self.ReceiveAnyDamage`
  (params (Damage :type "Float (single-precision)") (DamageType :type "DamageType Object Reference") (InstigatedBy :type "Controller Object Reference") (DamageCauser :type "Actor Object Reference"))
  (bind _slot_name (`self.Slot Name`))
  ;[1 1 1] CanBeDestroyed
  (bind _result (`/Engine/EditorBlueprintResources/StandardMacros.DecrementFloat` (`self.MaxHP`))
    (:`  `
      (set `self.CurrentHP` _result)
      (if (== 0.0 (`self.CurrentHP`))
        (`GameplayStatics.SpawnSound2D` "/Game/Sounds/enemydestroyed.enemydestroyed" 0.1 1.0 0.0 null false false)
        (bind _returnvalue (`GameplayStatics.LoadGameFromSlot` _slot_name))
        (bind _asbp_endles_save_game (cast `/Game/Widgets/BP_EndlesSaveGame` _returnvalue))
        (set `/Game/Widgets/BP_EndlesSaveGame.Coins` (+ (`/Game/Widgets/BP_EndlesSaveGame.Coins` _asbp_endles_save_game) (`self.PointSelf`)) _asbp_endles_save_game)
        (`GameplayStatics.SaveGameToSlot` _asbp_endles_save_game _slot_name)
        (`self.K2_DestroyActor`)
        (bind _output_get (set `self.ExplosionRandom` (`KismetMathLibrary.RandomIntegerInRange` 0 2)))
        (if (== _output_get 0)
          (`GameplayStatics.SpawnEmitterAtLocation` "/Game/Assets/M5VFXVOL2/Particles/Explosion/Fire_Exp_03.Fire_Exp_03" (`self.K2_GetActorLocation`))
          (elif (== (`self.ExplosionRandom`) 1)
            (`GameplayStatics.SpawnEmitterAtLocation` "/Game/Assets/M5VFXVOL2/Particles/Explosion/Fire_Exp_00.Fire_Exp_00" (`self.K2_GetActorLocation`))
            (elif (== (`self.ExplosionRandom`) 2)
              (`GameplayStatics.SpawnEmitterAtLocation` "/Game/Assets/M5VFXVOL2/Particles/Explosion/Fire_Exp_01.Fire_Exp_01" (`self.K2_GetActorLocation`)))))))))

(event `self.ReceiveActorBeginOverlap`
  (params (OtherActor :type "Actor Object Reference")))

(event `self.ReceiveBeginPlay`
  ;[1 1 1] Moving
  (set `self.CurrentHP` (`self.MaxHP`))
  (`AIController.RunBehaviorTree` (`AIBlueprintHelperLibrary.GetAIController` self) "/Game/Assets/Enemies/FlyingAIBT.FlyingAIBT"))

(event `self.Box.OnComponentBeginOverlap`
  (params (OverlappedComponent :type "PrimitiveComponent Object Reference") (OtherActor :type "Actor Object Reference") (OtherComp :type "PrimitiveComponent Object Reference") (OtherBodyIndex :type Integer) (bFromSweep :type Boolean) (SweepResult :type "HitResult Structure (by ref)"))
  ;[1 1 1] Destroy by hitting shield and station
  (`|ExecutionSequence`
    (:`then_0`
      (bind _asbp_shield (cast `/Game/Blueprints/BP_Shield` OtherActor))
      (if (not (== OtherActor (`self.GetOwner` _asbp_shield)))
        (`GameplayStatics.ApplyDamage` OtherActor 1.0 :!label _label)
        (`GameplayStatics.SpawnSound2D` "/Game/Sounds/enemydestroyed.enemydestroyed" 0.1 1.0 0.0 null false false)
        (`self.K2_DestroyActor`)
        (set `self.ExplosionRandom` (`KismetMathLibrary.RandomIntegerInRange` 0 2))
        (if (== (`self.ExplosionRandom`) 0)
          (`GameplayStatics.SpawnEmitterAtLocation` "/Game/Assets/M5VFXVOL2/Particles/Explosion/Fire_Exp_03.Fire_Exp_03" (`self.K2_GetActorLocation`))
          (elif (== (`self.ExplosionRandom`) 1)
            (`GameplayStatics.SpawnEmitterAtLocation` "/Game/Assets/M5VFXVOL2/Particles/Explosion/Fire_Exp_00.Fire_Exp_00" (`self.K2_GetActorLocation`))
            (elif (== (`self.ExplosionRandom`) 2)
              (`GameplayStatics.SpawnEmitterAtLocation` "/Game/Assets/M5VFXVOL2/Particles/Explosion/Fire_Exp_01.Fire_Exp_01" (`self.K2_GetActorLocation`)))))))
    (:`then_1`
      (bind _asspace_station (cast `/Game/Assets/Space/SpaceObjects/SpaceStation` OtherActor))
      (if (not (== OtherActor (`self.GetOwner` _asspace_station)))
        (goto _label)))))

(event `self.ReceiveTick`
  (params (DeltaSeconds :type "Float (single-precision)"))
  ;[1 1 1] Moving
  (`SceneComponent.K2_AddLocalRotation` (`self.StaticMesh`) (`KismetMathLibrary.NormalizedDeltaRotator` (`KismetMathLibrary.MakeRotator` 0.0 0.0 DeltaSeconds) (struct :`Yaw` 0.4)) false false))

(fn `GetActor`
  (returns (Actor :type "Actor Object Reference"))
  (return null))

(fn `GetShildHP`
  (returns (ShildHP :type "Float (double-precision)"))
  (return 0.0))

(fn `GetStationHP`
  (returns (StationHP :type "Float (double-precision)"))
  (return 0.0))

(fn `UserConstructionScript`)