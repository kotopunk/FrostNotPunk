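; BP_RockEnemy is an enemy actor that repeatedly fires projectiles and can be destroyed by damage.
; From BeginPlay, a self-calling Fire event spawns BP_ProjectileEnemy at its Scene transform after each Delay.
; Each damage event decrements MaxHP by one regardless of amount, copies it to CurrentHP, and at zero plays a sound, destroys the actor and spawns one of three random explosions.
; Projectile, station/shield HP and actor getters are empty stubs.
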(event `self.ReceiveBeginPlay`
  (`self.Fire`))

(event `Fire`
  (`|SpawnActorFromClass` "/Game/Blueprints/BP_ProjectileEnemy.BP_ProjectileEnemy_C" (`SceneComponent.K2_GetComponentToWorld` (`self.Scene`)) "Undefined" "OverrideRootScale" self null)
  (`KismetSystemLibrary.Delay` (`self.Duration`))
  (`self.Fire`))

(event `self.ReceiveAnyDamage`
  (params (Damage :type "Float (single-precision)") (DamageType :type "DamageType Object Reference") (InstigatedBy :type "Controller Object Reference") (DamageCauser :type "Actor Object Reference"))
  (bind _result (`/Engine/EditorBlueprintResources/StandardMacros.DecrementFloat` (`self.MaxHP`))
    (:`  `
      (set `self.CurrentHP` _result)
      (if (== 0.0 (`self.CurrentHP`))
        (`GameplayStatics.SpawnSound2D` "/Game/Sounds/enemydestroyed.enemydestroyed" 0.1 1.0 0.0 null false false)
        (`self.K2_DestroyActor`)
        (bind _output_get (set `self.ExplosionRandom` (`KismetMathLibrary.RandomIntegerInRange` 0 2)))
        (if (== _output_get 0)
          (`GameplayStatics.SpawnEmitterAtLocation` "/Game/Assets/M5VFXVOL2/Particles/Explosion/Fire_Exp_03.Fire_Exp_03" (`self.K2_GetActorLocation`))
          (elif (== (`self.ExplosionRandom`) 1)
            (`GameplayStatics.SpawnEmitterAtLocation` "/Game/Assets/M5VFXVOL2/Particles/Explosion/Fire_Exp_00.Fire_Exp_00" (`self.K2_GetActorLocation`))
            (elif (== (`self.ExplosionRandom`) 2)
              (`GameplayStatics.SpawnEmitterAtLocation` "/Game/Assets/M5VFXVOL2/Particles/Explosion/Fire_Exp_01.Fire_Exp_01" (`self.K2_GetActorLocation`)))))))))

(fn `GetActor`
  (returns (Actor :type "Actor Object Reference"))
  (return null))

(fn `GetShildHP`
  (returns (ShildHP :type "Float (double-precision)"))
  (return 0.0))

(fn `GetStationHP`
  (returns (StationHP :type "Float (double-precision)"))
  (return 0.0))

(fn `Projectile`
  (returns (Damage :type "Float (double-precision)"))
  (return 0.0))

(fn `UserConstructionScript`)